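; BP_Sword is a sword weapon actor that exposes its combat data to other code.
; Getters return its damage, montage, trace radius and the world locations of two components marking the trace start and end.
; The PickUp event only prints "Sword", and the asset runs no traces or damage logic itself.
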(event `/Game/Blueprint/Interfaces/BPI_Pickable.PickUp`
  (`KismetSystemLibrary.PrintString` "Sword"))

(fn `GetDamage`
  (returns (Damage :type "Float (double-precision)"))
  (return (`self.Damage`)))

(fn `GetTraceRadious`
  (returns (TraceRadious :type "Float (double-precision)"))
  (return (`self.TraceRadious`)))

(fn `GetWeponMontage`
  (returns (WeponAnimMontage :type "AnimMontage Object Reference"))
  (return (`self.WeponMontage`)))

(fn `GetWeponTraceEnd`
  (returns (TraceEnd :type "Vector Structure"))
  (return (`SceneComponent.K2_GetComponentLocation` (`self.TraceEndPosition`))))

(fn `GetWeponTraceStart`
  (returns (TraceStart :type "Vector Structure"))
  (return (`SceneComponent.K2_GetComponentLocation` (`self.traceStartPosition`))))

(fn `UserConstructionScript`)