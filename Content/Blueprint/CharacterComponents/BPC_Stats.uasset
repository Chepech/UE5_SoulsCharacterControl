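; Character stats component that holds Health, Strength, Agility, Intelligence and Eldrich values.
; Health starts at MaxHealth on BeginPlay, and GetStat reads any stat through a switch on the stat type.
; ModifyStat adds a signed change to the chosen stat, clamping only Health between zero and MaxHealth.
; Its return value adds the change again to the updated stat, so it can differ from the stored value.
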(event `self.ReceiveBeginPlay`
  ; Set Defaults
  (set `self.Health` (`self.MaxHealth`)))

(fn `GetStat`
  (params (Stat :type "/Game/Blueprint/CharacterComponents/ENUM_Stats Enum" :default "NewEnumerator0"))
  (returns (statValue :type "Float (double-precision)"))
  (locals (localStatValue :type "Float (double-precision)"))
  (switch `/Game/Blueprint/CharacterComponents/ENUM_Stats` Stat
    (:`NewEnumerator0`
      (set `local.localStatValue` (`self.Health`)))
    (:`NewEnumerator1`
      (set `local.localStatValue` (`self.Strength`)))
    (:`NewEnumerator2`
      (set `local.localStatValue` (`self.Agility`)))
    (:`NewEnumerator3`
      (set `local.localStatValue` (`self.Inteligence`)))
    (:`NewEnumerator4`
      (set `local.localStatValue` (`self.Eldrich`))))
  (return (`local.localStatValue`)))

(fn `ModifyStat`
  (params (Stat :type "/Game/Blueprint/CharacterComponents/ENUM_Stats Enum" :default "NewEnumerator0") (value :type "Float (double-precision)"))
  (returns (NewStatValue :type "Float (double-precision)"))
  (locals (statChangeAmmount :type "Float (double-precision)") (statValue :type "Float (double-precision)"))
  (bind _returnvalue (+ (`self.Eldrich`) (`local.statChangeAmmount`)))
  (bind _returnvalue_2 (+ (`self.Strength`) (`local.statChangeAmmount`)))
  (bind _returnvalue_3 (+ (`self.Agility`) (`local.statChangeAmmount`)))
  (bind _returnvalue_4 (+ (`self.Inteligence`) (`local.statChangeAmmount`)))
  (bind _returnvalue_5 (`KismetMathLibrary.FClamp` (+ (`self.Health`) (`local.statChangeAmmount`)) 0.0 (`self.MaxHealth`)))
  (set `local.statChangeAmmount` value)
  (switch `/Game/Blueprint/CharacterComponents/ENUM_Stats` Stat
    (:`NewEnumerator0`
      ; Health
      (set `self.Health` _returnvalue_5)
      (set `local.statValue` _returnvalue_5))
    (:`NewEnumerator1`
      ; Strength
      (set `self.Strength` _returnvalue_2)
      (set `local.statValue` _returnvalue_2))
    (:`NewEnumerator2`
      ; Agility
      (set `self.Agility` _returnvalue_3)
      (set `local.statValue` _returnvalue_3))
    (:`NewEnumerator3`
      ; Intelligence
      (set `self.Inteligence` _returnvalue_4)
      (set `local.statValue` _returnvalue_4))
    (:`NewEnumerator4`
      ; Eldrich
      (set `self.Eldrich` _returnvalue)
      (set `local.statValue` _returnvalue)))
  (return (`local.statValue`)))