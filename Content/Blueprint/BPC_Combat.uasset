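; Player combat component that adds hold-to-lock targeting and a sword combo attack to the third-person character.
; Holding IA_Lock sphere-traces along the camera direction, attaches a marker to the hit actor and switches movement to controller-driven strafing.
; While locked, Tick turns the control rotation toward that target.
; IA_Attack plays a combo montage, which stops at each notify unless another press has queued the next hit.
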(event `self.ReceiveBeginPlay`
  ; Init
  (set `self.CameraManager` (`GameplayStatics.GetPlayerCameraManager` 0))
  (bind _asbp_third_person_character (cast `/Game/ThirdPerson/Blueprints/BP_ThirdPersonCharacter` (`GameplayStatics.GetPlayerPawn` 0)))
  (bind _output_get (set `self.PlayerPawn` _asbp_third_person_character))
  (set `self.CharacterMovement` (`Character.CharacterMovement` _output_get)))

(event `self.ReceiveTick`
  (params (DeltaSeconds :type "Float (single-precision)"))
  (bind (_returnvalue_x _returnvalue_y _returnvalue_z) (`KismetMathLibrary.BreakVector` (`Actor.K2_GetActorLocation` (`self.DetectedActor`))))
  ; Strafe when con Combat
  ; Force controller to point to detected Enemy Pawn
  (if (`self.isOnCombat`)
    (`self.DetectedActor`
      (:`then`
        (`Controller.SetControlRotation` (`Pawn.GetController` (`self.PlayerPawn`)) (`KismetMathLibrary.RLerp` (`Actor.K2_GetActorRotation` (`self.PlayerPawn`)) (`KismetMathLibrary.FindLookAtRotation` (`Actor.K2_GetActorLocation` (`self.PlayerPawn`)) (`KismetMathLibrary.MakeVector` _returnvalue_x _returnvalue_y (+ _returnvalue_z -200.0))) DeltaSeconds true)))
      (:`else`))))

(event `EnhancedInput|/Game/ThirdPerson/Input/Actions/IA_Lock`
  (params (ActionValue :type Boolean) (ElapsedSeconds :type "Float (double-precision)") (TriggeredSeconds :type "Float (double-precision)") (InputAction :type "InputAction Object Reference" :default "/Game/ThirdPerson/Input/Actions/IA_Lock.IA_Lock"))
  (:`Started`
    ; Trace and Detect Pawns to Lock rotation to and add a marker to the found character
    (bind (_detectedenemy _wasenemydetected) (`self.DetectEnemy`))
    (if _wasenemydetected
      (bind _output_get (set `self.DetectedActor` _detectedenemy))
      (`self.StartCombatMovementMode`)
      (bind _returnvalue (`Actor.GetTransform` _output_get))
      (bind _returnvalue_2 (`|SpawnActorFromClass` "/Game/UI/Props/BP_TargetedMarker.BP_TargetedMarker_C" (`KismetMathLibrary.MakeTransform` (`KismetMathLibrary.MakeVector` (.x (.location _returnvalue)) (.y (.location _returnvalue)) (+ (.z (.location _returnvalue)) (`self.TargetMarkerOffsetZ`))) (.rotation _returnvalue) (.scale _returnvalue)) "AlwaysSpawn" "MultiplyWithRoot" (`self.DetectedActor`) null))
      (bind _output_get_2 (set `self.SpawnnedTargetMarker` _returnvalue_2))
      (`Actor.K2_AttachToActor` _output_get_2 (`self.DetectedActor`) "None" "KeepWorld" "KeepWorld" "KeepRelative" true)))
  (:`Completed`
    (`self.StopCombatMovementMode`)
    (bind _spawnnedtargetmarker (`self.SpawnnedTargetMarker`)
      (:`then`
        (`Actor.K2_DestroyActor` _spawnnedtargetmarker))
      (:`else`))))

(event `EnhancedInput|/Game/ThirdPerson/Input/Actions/IA_Attack`
  (params (ActionValue :type Boolean) (ElapsedSeconds :type "Float (double-precision)") (TriggeredSeconds :type "Float (double-precision)") (InputAction :type "InputAction Object Reference" :default "/Game/ThirdPerson/Input/Actions/IA_Attack.IA_Attack"))
  (:`Started`
    ; Attack
    (if (not (`self.IsAttacking`))
      (`|PlayMontage` (`Character.Mesh` (`self.PlayerPawn`)) "/Game/Characters/Animations/CombatLocomotion/SwordAttackCombo_Anim_Montage.SwordAttackCombo_Anim_Montage"
        (:`then`
          (set `self.IsAttacking` true)
          (set `self.isComboAttack` false :!label _label))
        (:`OnCompleted`
          (set `self.IsAttacking` false :!label _label_2)
          (goto _label))
        (:`OnInterrupted`
          (goto _label_2))
        (:`OnNotifyBegin`
          (if (and (`self.IsAttacking`) (`self.isComboAttack`))
            (goto _label)
            (else
              (`AnimInstance.Montage_Stop` (`SkeletalMeshComponent.GetAnimInstance` (`Character.Mesh` (`self.PlayerPawn`))) 0.2 "/Game/Characters/Animations/CombatLocomotion/SwordAttackCombo_Anim_Montage.SwordAttackCombo_Anim_Montage")))))
      (else
        (set `self.isComboAttack` true)))))

(fn `DetectEnemy`
  (returns (DetectedEnemy :type "Actor Object Reference") (wasEnemyDetected :type Boolean))
  (bind (_start _end) (`self.GetFromPawnTrace`))
  (bind (_outhit _returnvalue) (`KismetSystemLibrary.SphereTraceSingleForObjects` _start _end 300.0 (`self.VisibleObjectTypes`) false (`self.IgnoreObjects`) "ForDuration" true (struct :`R` 1.0 :`A` 1.0) (struct :`G` 1.0 :`A` 1.0) 2.0))
  (if _returnvalue
    _
    (else
      _))
  (return (`.HitActor` (`GameplayStatics.BreakHitResult` _outhit)) _returnvalue))

(fn `GetFromPawnTrace`
  (returns (Start :type "Vector Structure") (End :type "Vector Structure"))
  (bind _returnvalue (`Actor.K2_GetActorLocation` (`self.PlayerPawn`)))
  (return _returnvalue (+ _returnvalue (* (`KismetMathLibrary.GetForwardVector` (`PlayerCameraManager.GetCameraRotation` (`self.CameraManager`))) (`self.LookDistance`)))))

(fn `StartCombatMovementMode`
  (bind _charactermovement (`self.CharacterMovement`))
  (set `CharacterMovementComponent.bOrientRotationToMovement` false _charactermovement)
  (set `CharacterMovementComponent.bUseControllerDesiredRotation` true _charactermovement)
  (set `self.isOnCombat` true))

(fn `StopCombatMovementMode`
  (bind _charactermovement (`self.CharacterMovement`))
  (set `CharacterMovementComponent.bOrientRotationToMovement` true _charactermovement)
  (set `CharacterMovementComponent.bUseControllerDesiredRotation` false _charactermovement)
  (set `self.isOnCombat` false))